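; Interactive sliding door actor that lowers to open and rises to close when the first-person character presses Interact nearby.
; A Sensor overlap enables input and shows front and rear text prompts.
; MoveComponentTo animates the door while both lights and prompts reflect its state.
; A broken door only drops partway and springs back, and the construction script previews the IsDoorOpen starting state.
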(event OnComponentBeginOverlap(Sensor)
  (params (OverlappedComponent :type Primitive%20Component%20Object%20Reference) (OtherActor :type Actor%20Object%20Reference) (OtherComp :type Primitive%20Component%20Object%20Reference) (OtherBodyIndex :type Integer) (bFromSweep :type Boolean) (SweepResult :type Hit%20Result%20Structure%20%28by%20ref%29))
  (if (== (Utilities|GetClass OtherActor) "/Game/FirstPerson/Blueprints/BP_FirstPersonCharacter.BP_FirstPersonCharacter_C")
    (Input|EnableInput (Game|GetPlayerController 0))
    (Rendering|SetVisibility (Variables|Default|GetTextPromptFront) true false)))

(event OnComponentEndOverlap(Sensor)
  (params (OverlappedComponent :type Primitive%20Component%20Object%20Reference) (OtherActor :type Actor%20Object%20Reference) (OtherComp :type Primitive%20Component%20Object%20Reference) (OtherBodyIndex :type Integer))
  (if (== (Utilities|GetClass OtherActor) "/Game/FirstPerson/Blueprints/BP_FirstPersonCharacter.BP_FirstPersonCharacter_C")
    (Input|DisableInput (Game|GetPlayerController 0))
    (Rendering|SetVisibility (Variables|Default|GetTextPromptRear) false false)))

(event Custom|CloseDoor
  (Rendering|SetVisibility (Variables|Default|GetTextPromptRear) false false)
  (Rendering|Components|Light|SetLightColor (Variables|Default|GetRearLight) "(R=1.000000,G=0.392157,B=0.000000,A=1.000000)" true)
  (Components|MoveComponentTo (Variables|Default|GetDoor) (Variables|Default|GetOriginalLocation) "0, 0, 0" false false 1.0 false)
  (Rendering|SetVisibility (Variables|Default|GetTextPromptRear) true false)
  (Variables|Default|SetIsDoorOpen false)
  (Rendering|Components|Light|SetLightColor (Variables|Default|GetForwardLight) "(R=1.000000,G=0.000000,B=0.000000,A=1.000000)" true)
  (Rendering|Components|TextRender|SetText (Variables|Default|GetTextPromptRear) (Utilities|Text|FormatText "Press \"E\" To Open")))

(event Custom|OpenDoor
  (Rendering|SetVisibility (Variables|Default|GetTextPromptRear) false false)
  (Rendering|Components|Light|SetLightColor (Variables|Default|GetRearLight) "(R=1.000000,G=0.392157,B=0.000000,A=1.000000)" true)
  (Components|MoveComponentTo (Variables|Default|GetDoor) (+ (Variables|Default|GetOriginalLocation) "0.000000,0.000000,-150.000000") "0, 0, 0" false false 1.0 false)
  (Rendering|SetVisibility (Variables|Default|GetTextPromptRear) true false)
  (Variables|Default|SetIsDoorOpen true)
  (Rendering|Components|Light|SetLightColor (Variables|Default|GetRearLight) "(R=0.014428,G=1.000000,B=0.000000,A=1.000000)" true)
  (Rendering|Components|TextRender|SetText (Variables|Default|GetTextPromptFront) (Utilities|Text|FormatText "Press \"E\" To Close")))

(event Custom|BrokenDoor
  (Rendering|SetVisibility (Variables|Default|GetTextPromptRear) false false)
  (Rendering|Components|Light|SetLightColor (Variables|Default|GetRearLight) "(R=1.000000,G=0.392157,B=0.000000,A=1.000000)" true)
  (Components|MoveComponentTo (Variables|Default|GetDoor) (+ (Variables|Default|GetOriginalLocation) "0.000000,0.000000,-40.000000") "0, 0, 0" false false 1.0 false)
  (Utilities|FlowControl|Delay 1.0)
  (Components|MoveComponentTo (Variables|Default|GetDoor) (Variables|Default|GetOriginalLocation) "0, 0, 0" false false 1.0 false)
  (Rendering|SetVisibility (Variables|Default|GetTextPromptRear) true false)
  (Variables|Default|SetIsDoorOpen false)
  (Rendering|Components|Light|SetLightColor (Variables|Default|GetRearLight) "(R=1.000000,G=0.000000,B=0.048679,A=1.000000)" true)
  (Rendering|Components|TextRender|SetText (Variables|Default|GetTextPromptFront) (Utilities|Text|FormatText "Press \"E\" To Open?")))

(event EventBeginPlay)

(event Collision|EventActorBeginOverlap
  (params (OtherActor :type Actor%20Object%20Reference)))

(event EventTick
  (params (DeltaSeconds :type Float%20%28single-precision%29)))

(event Input|ActionEvents|InputActionInteract
  (params (Key :type Key%20Structure :default "None"))
  (:Pressed
    (if (Variables|Default|GetIsDoorBroken)
      (CallFunction|BrokenDoor)
      (elif (Variables|Default|GetIsDoorOpen)
        (CallFunction|CloseDoor)
        (else
          (CallFunction|OpenDoor))))))

(fn ConstructionScript
  (Variables|Default|SetOriginalLocation (Variables|/Script/Engine.SceneComponent|GetRelativeLocation (Variables|Default|GetDoor)))
  (if (Variables|Default|GetIsDoorOpen)
    (Transformation|SetRelativeLocation (Variables|Default|GetDoor) (+ (Variables|Default|GetOriginalLocation) "0.000000,0.000000,-150.000000") false false)
    (Rendering|Components|Light|SetLightColor (Variables|Default|GetRearLight) "(R=0.014428,G=1.000000,B=0.000000,A=1.000000)" true)
    (Rendering|Components|TextRender|SetText (Variables|Default|GetTextPromptFront) (Utilities|Text|FormatText "Press \"E\" To Close"))
    (else
      (Rendering|Components|Light|SetLightColor (Variables|Default|GetForwardLight) "(R=1.000000,G=0.000000,B=0.000000,A=1.000000)" true)
      (Rendering|Components|TextRender|SetText (Variables|Default|GetTextPromptRear) (Utilities|Text|FormatText "Press \"E\" To Open")))))